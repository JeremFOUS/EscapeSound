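; Audio actor that keeps a close-sea ambience sound on the point of its spline nearest the player, so the sea sound follows along that path.
; On BeginPlay it caches the player's BP_ThirdPersonCharacter, then starts MoveAudio.
; MoveAudio moves the AMBSeaClose component to the closest spline location with a small upward offset, then re-calls itself after a short Delay, looping instead of using Tick.
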(event Custom|Move%20Audio
  (bind _char_ref (Variables|Default|GetChar%20REF))
  (bind _spline (Variables|Default|GetSpline))
  (bind _returnvalue (Transformation|GetActorLocation _char_ref))
  (bind _returnvalue_2 (Spline|FindLocationClosesttoWorldLocation _spline _returnvalue "World"))
  (Transformation|SetWorldLocation (Variables|Default|GetAMB_Sea_Close) (Math|Vector|MakeVector (.x _returnvalue_2) (.y _returnvalue_2) (+ (.z _returnvalue_2) 5e+01)) false false)
  (Utilities|FlowControl|Delay 0.05)
  (CallFunction|MoveAudio))

(event EventBeginPlay
  (bind _asbp_third_person_character (Utilities|Casting|CastToBP_ThirdPersonCharacter (Game|GetPlayerCharacter 0)))
  (Variables|Default|SetChar%20REF _asbp_third_person_character)
  (CallFunction|MoveAudio))

(event Collision|EventActorBeginOverlap
  (params (OtherActor :type Actor%20Object%20Reference)))

(event EventTick
  (params (DeltaSeconds :type Float%20%28single-precision%29)))

(fn ConstructionScript)