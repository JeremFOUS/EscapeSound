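; A door actor that swings open when interacted with.
; It records its starting rotation on BeginPlay.
; Interact plays an Opening timeline that lerps the actor's yaw to 90 degrees below that rotation, and an event track on it plays an attenuated door-open sound at the actor's location.
; There is no closing logic.
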(event EventBeginPlay
  (Variables|Default|SetStartingRotation (Transformation|GetActorRotation)))

(event EventInteract
  (bind _startingrotation (Variables|Default|GetStartingRotation))
  (bind _newtrack_0 (Timeline|Opening Play)
    (:Update
      (Transformation|SetActorRotation (Math|Rotator|Lerp(Rotator) (Variables|Default|GetStartingRotation) (Math|Rotator|MakeRotator (.roll _startingrotation) (.pitch _startingrotation) (+ (.yaw _startingrotation) -9e+01)) _newtrack_0 true)))
    (:Play_Door
      (Audio|PlaySoundatLocation "/Game/AUDIO/SoundBank/SFX/SFX_DoorOpen_01.SFX_DoorOpen_01" (Transformation|GetActorLocation) "0, 0, 0" 0.35 1.0 0.0 "/Game/AUDIO/Attenuation/ATT_Door.ATT_Door" 0 0 0))))

(fn ConstructionScript)